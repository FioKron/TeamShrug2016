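; BP_Score is a Blueprint that handles the player's death by clearing the HUD and hiding the character.
; BeginPlay caches the FirstPersonCharacter and the first BP_Spawner and BP_Timer found in the level.
; Tick polls the player's IsDead flag, then zeroes the timer's Milliseconds, clears the flag, removes PlayerHUD and hides the player.
; Despite the name, it holds no score logic, and the spawner reference goes unused.
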(event EventTick
  (params (DeltaSeconds :type Float%20%28single-precision%29))
  (bind _player (Variables|Default|GetPlayer))
  ;[1 1 1] Remove current HUD
  (if (Variables|/Game/Blueprints/FirstPersonCharacter.FirstPersonCharacter_C|GetisDead (Variables|Default|GetPlayer))
    (Variables|/Game/Blueprints/BP_Timer.BP_Timer_C|SetMilliseconds (Variables|Default|GetTimer) 0)
    (Variables|/Game/Blueprints/FirstPersonCharacter.FirstPersonCharacter_C|SetisDead _player false)
    (Widget|RemovefromParent (Variables|/Game/Blueprints/FirstPersonCharacter.FirstPersonCharacter_C|GetPlayer_HUD _player))
    (Rendering|SetActorHiddenInGame (Variables|Default|GetPlayer) true)))

(event EventBeginPlay
  ;[1 1 1] References
  (bind _asfirst_person_character (Utilities|Casting|CastToFirstPersonCharacter (Game|GetPlayerCharacter 0)))
  (Variables|Default|SetPlayer _asfirst_person_character)
  (bind _outactors (Actor|GetAllActorsOfClass "/Game/Blueprints/BP_Spawner.BP_Spawner_C"))
  (Variables|Default|SetSpawner (Utilities|Array|Get(acopy) _outactors))
  (bind _outactors_2 (Actor|GetAllActorsOfClass "/Game/Blueprints/BP_Timer.BP_Timer_C"))
  (Variables|Default|SetTimer (Utilities|Array|Get(acopy) _outactors_2)))

(fn ConstructionScript)