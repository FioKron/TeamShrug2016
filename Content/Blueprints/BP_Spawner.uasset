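; BP_Spawner scatters BP_Mine actors across the level's TargetPoints when play begins.
; A BeginPlay loop runs until MineCount reaches TotalMines, each pass gathering all TargetPoints and picking a random index to spawn a mine at that location.
; Each used TargetPoint is destroyed after spawning, removing it as a candidate for later mines.
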(event EventBeginPlay
  ;[1 1 1] Spawning
  (while (<= (Variables|Default|GetMineCount) (- (Variables|Default|GetTotal%20Mines) 1))
    (bind _outactors (Actor|GetAllActorsOfClass "/Script/Engine.TargetPoint"))
    (bind _output_get (Variables|Default|SetSpawnPointNumber (Math|Random|RandomInteger (- (Utilities|Array|Length _outactors) 1))))
    (Game|SpawnActorfromClass "/Game/Blueprints/BP_Mine.BP_Mine_C" (Math|Conversions|ToTransform(Vector) (Transformation|GetActorLocation (Utilities|Array|Get(acopy) _outactors _output_get))) "Undefined" 0 0)
    (Actor|DestroyActor (Utilities|Array|Get(acopy) _outactors _output_get))
    (Math|Integer|IncrementInt (Variables|Default|GetMineCount))))

(fn ConstructionScript)